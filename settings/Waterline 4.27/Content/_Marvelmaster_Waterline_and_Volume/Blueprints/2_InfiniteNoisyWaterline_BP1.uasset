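; Infinite noisy waterline actor that, while MakeInfinite is on, keeps its water plane centered under or over the player camera.
; Each tick it snaps to the camera's XY at a fixed height and writes that position and the mesh extent to WaterMask_MPC as the water mask.
; A DoOnce resets those parameters to large defaults when infinite mode is off, as does the construction script.
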(event `self.ReceiveBeginPlay`
  (set `self.Initial Location` (`self.K2_GetActorLocation`)))

(event `self.ReceiveTick`
  (params (DeltaSeconds :type "Float (single-precision)"))
  (bind _returnvalue (`KismetMathLibrary.Conv_DoubleToLinearColor` (* 1.0 100000.0)))
  (bind (_returnvalue_x _returnvalue_y) (`KismetMathLibrary.BreakVector` (`PlayerCameraManager.GetCameraLocation` (`PlayerController.PlayerCameraManager` (`GameplayStatics.GetPlayerController` 0)))))
  (if (`self.MakeInfinite`)
    ;[1 1 1] set water plane mesh to the actor location and write the location and waterplane size to the material parameter collection
    (`self.K2_SetActorLocation` (`KismetMathLibrary.MakeVector` _returnvalue_x _returnvalue_y 1000.0))
    (`KismetMaterialLibrary.SetVectorParameterValue` "/Game/_Marvelmaster_Waterline_and_Volume/MaterialFunction+Collections/WaterMask_MPC.WaterMask_MPC" "CameraLoc" (`KismetMathLibrary.Conv_VectorToLinearColor` (`KismetMathLibrary.MakeVector` _returnvalue_x _returnvalue_y)))
    (`KismetMaterialLibrary.SetVectorParameterValue` "/Game/_Marvelmaster_Waterline_and_Volume/MaterialFunction+Collections/WaterMask_MPC.WaterMask_MPC" "MaskSize" (`KismetMathLibrary.Conv_VectorToLinearColor` (`.BoxExtent` (`KismetSystemLibrary.GetComponentBounds` (`self.StaticMesh`)))))
    (goto _label :!via `Reset`)
    (else
      ;[1 1 1] reset parameters when not infinite
      (`/Engine/EditorBlueprintResources/StandardMacros.DoOnce` false :!label _label
        (:`Completed`
          (`KismetMaterialLibrary.SetVectorParameterValue` "/Game/_Marvelmaster_Waterline_and_Volume/MaterialFunction+Collections/WaterMask_MPC.WaterMask_MPC" "CameraLoc" _returnvalue)
          (`KismetMaterialLibrary.SetVectorParameterValue` "/Game/_Marvelmaster_Waterline_and_Volume/MaterialFunction+Collections/WaterMask_MPC.WaterMask_MPC" "MaskSize" _returnvalue))))))

(fn `UserConstructionScript`
  (bind _returnvalue (`KismetMathLibrary.Conv_DoubleToLinearColor` (* 1.0 100000.0)))
  ;[1 1 1] this is only for infinite waterline, reset the parameters on spawn
  (`KismetMaterialLibrary.SetVectorParameterValue` "/Game/_Marvelmaster_Waterline_and_Volume/MaterialFunction+Collections/WaterMask_MPC.WaterMask_MPC" "CameraLoc" _returnvalue)
  (`KismetMaterialLibrary.SetVectorParameterValue` "/Game/_Marvelmaster_Waterline_and_Volume/MaterialFunction+Collections/WaterMask_MPC.WaterMask_MPC" "MaskSize" _returnvalue))