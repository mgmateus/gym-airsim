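; Water volume Blueprint that drives a waterline effect through a scene capture attached to the player camera.
; The capture's show-only list holds the waterline cube and blocks, which owner-no-see hides from the player.
; Overlapping the cube toggles player mesh custom depth, while an outer box shows or hides the capture by range.
; Construction greatly enlarges the cube, plane and top block bounds against flicker.
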(event `self.ReceiveBeginPlay`
  (`|ExecutionSequence`
    (:`then_0`
      ;[1 1 1] show only some objects to scene capture, but hide these object from player
      (for _array_element (`|MakeArray` (`self.WaterlineCube`) (`self.BlockTop`) (`self.BlockBottom`) :!type "PrimitiveComponent Object Reference")
        (`SceneCaptureComponent.ShowOnlyComponent` (`self.SceneCaptureComponent2D`) _array_element))
      (`self.SetOwner` (`GameplayStatics.GetPlayerCharacter` 0))
      (`PrimitiveComponent.SetOwnerNoSee` (`self.BlockBottom`) true)
      (`PrimitiveComponent.SetOwnerNoSee` (`self.BlockTop`) true)
      (`PrimitiveComponent.SetOwnerNoSee` (`self.WaterlineCube`) true))
    (:`then_1`
      ;[1 1 1] Attach scene capture to camera
      (`SceneComponent.K2_AttachToComponent` (`self.SceneCaptureComponent2D`) (`PlayerCameraManager.TransformComponent` (`PlayerController.PlayerCameraManager` (`GameplayStatics.GetPlayerController` 0))) "None" "SnapToTarget" "SnapToTarget" "SnapToTarget" true))))

(event `self.WaterlineCube.OnComponentBeginOverlap`
  (params (OverlappedComponent :type "PrimitiveComponent Object Reference") (OtherActor :type "Actor Object Reference") (OtherComp :type "PrimitiveComponent Object Reference") (OtherBodyIndex :type Integer) (bFromSweep :type Boolean) (SweepResult :type "HitResult Structure (by ref)"))
  ;[1 1 1] Flip character custom depht depending on char overlap (MUST be activated by hand the char mesh first!!)
  (`PrimitiveComponent.SetRenderCustomDepth` (`Character.Mesh` (`GameplayStatics.GetPlayerCharacter` 0)) false)
  (`KismetSystemLibrary.PrintString` "Custom Depth disabled"))

(event `self.WaterlineCube.OnComponentEndOverlap`
  (params (OverlappedComponent :type "PrimitiveComponent Object Reference") (OtherActor :type "Actor Object Reference") (OtherComp :type "PrimitiveComponent Object Reference") (OtherBodyIndex :type Integer))
  ;[1 1 1] Flip character custom depht depending on char overlap (MUST be activated by hand the char mesh first!!)
  (`PrimitiveComponent.SetRenderCustomDepth` (`Character.Mesh` (`GameplayStatics.GetPlayerCharacter` 0)) true)
  (`KismetSystemLibrary.PrintString` "Hello"))

(event `self.Box.OnComponentBeginOverlap`
  (params (OverlappedComponent :type "PrimitiveComponent Object Reference") (OtherActor :type "Actor Object Reference") (OtherComp :type "PrimitiveComponent Object Reference") (OtherBodyIndex :type Integer) (bFromSweep :type Boolean) (SweepResult :type "HitResult Structure (by ref)"))
  ;[1 1 1] deactivate capture when out of range, capture is initially hidden in BP
  (`SceneComponent.SetHiddenInGame` (`self.SceneCaptureComponent2D`) false false))

(event `self.Box.OnComponentEndOverlap`
  (params (OverlappedComponent :type "PrimitiveComponent Object Reference") (OtherActor :type "Actor Object Reference") (OtherComp :type "PrimitiveComponent Object Reference") (OtherBodyIndex :type Integer))
  ;[1 1 1] deactivate capture when out of range, capture is initially hidden in BP
  (`SceneComponent.SetHiddenInGame` (`self.SceneCaptureComponent2D`) true false))

(fn `UserConstructionScript`
  ;[1 1 1] Flicker Debug
  (`PrimitiveComponent.SetBoundsScale` (`self.WaterlineCube`) 10000.0)
  (`PrimitiveComponent.SetBoundsScale` (`self.WaterPlane`) 10000.0)
  (`PrimitiveComponent.SetBoundsScale` (`self.BlockTop`) 10000.0))